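; Player character Blueprint that handles movement, look rotation and drone spawning through Enhanced Input.
; On possession it adds the IMC_Character mapping context, then movement input follows the control rotation's forward and right vectors while rotation actions drive controller yaw and pitch.
; The drone spawn action creates a BP_Drone a fixed distance in front of player 0's pawn, copying its rotation and scale, with this character as instigator.
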(event Input|EnhancedActionEvents|EnhancedInputActionIA_DroneSpawn
  (params (ActionValue :type Boolean) (ElapsedSeconds :type Float%20%28double-precision%29) (TriggeredSeconds :type Float%20%28double-precision%29) (InputAction :type Input%20Action%20Object%20Reference :default "/Game/Input/IA_DroneSpawn.IA_DroneSpawn"))
  (bind _returnvalue (Game|Player|GetPlayerPawn 0))
  (bind _returnvalue_2 (Transformation|GetActorTransform _returnvalue))
  (bind (_location _rotation _scale) (Math|Transform|BreakTransform _returnvalue_2))
  (:Triggered
    (Game|SpawnActorfromClass "/Game/Blueprints/BP_Drone.BP_Drone_C" (Math|Transform|MakeTransform (+ (* (Transformation|GetActorForwardVector _returnvalue) 3e+02) _location) _rotation _scale) "Undefined" "MultiplyWithRoot" 0 self)))

(event Input|EnhancedActionEvents|EnhancedInputActionIA_Move
  (params (ActionValue :type Vector%202D%20Structure) (ElapsedSeconds :type Float%20%28double-precision%29) (TriggeredSeconds :type Float%20%28double-precision%29) (InputAction :type Input%20Action%20Object%20Reference :default "/Game/Input/IA_Move.IA_Move"))
  ;[1 1 1] 이동, 회전
  (:Triggered
    (Pawn|Input|AddMovementInput (Math|Vector|GetRightVector (Pawn|GetControlRotation :!class /Script/Engine.Pawn)) (.x ActionValue) false)
    (Pawn|Input|AddMovementInput (Math|Vector|GetForwardVector (Pawn|GetControlRotation :!class /Script/Engine.Pawn)) (.y ActionValue) false)))

(event Input|EnhancedActionEvents|EnhancedInputActionIA_Rotation_X
  (params (ActionValue :type Float%20%28double-precision%29) (ElapsedSeconds :type Float%20%28double-precision%29) (TriggeredSeconds :type Float%20%28double-precision%29) (InputAction :type Input%20Action%20Object%20Reference :default "/Game/Input/IA_Rotation_X.IA_Rotation_X"))
  ;[1 1 1] 이동, 회전
  (:Triggered
    (Pawn|Input|AddControllerYawInput ActionValue)))

(event Input|EnhancedActionEvents|EnhancedInputActionIA_Rotation_Y
  (params (ActionValue :type Float%20%28double-precision%29) (ElapsedSeconds :type Float%20%28double-precision%29) (TriggeredSeconds :type Float%20%28double-precision%29) (InputAction :type Input%20Action%20Object%20Reference :default "/Game/Input/IA_Rotation_Y.IA_Rotation_Y"))
  ;[1 1 1] 이동, 회전
  (:Triggered
    (Pawn|Input|AddControllerPitchInput ActionValue)))

(event EventPossessed
  (params (NewController :type Controller%20Object%20Reference))
  ;[1 1 1] Enhanced Input
  (bind _asplayer_controller (Utilities|Casting|CastToPlayerController (Pawn|GetController)))
  (Input|AddMappingContext (PlayerController|LocalPlayerSubsystems|GetEnhancedInputLocalPlayerSubsystem _asplayer_controller) "/Game/Input/IMC_Character.IMC_Character" 0 "(bIgnoreAllPressedKeysUntilRelease=True,bForceImmediately=False)"))

(fn ConstructionScript)